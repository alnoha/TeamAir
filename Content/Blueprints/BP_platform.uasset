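; Platform actor that collapses piece by piece on a fixed timeline starting at BeginPlay.
; One hardcoded Delay and MoveComponentTo chain moves LandScapeSphere components to a shared LocationZ over Falltime, spaced by DelayPerFallingobject.
; Pieces drop in three waves separated by long pauses, with CamerashakeMessage sent to player 0 before the first two.
; The long final wave repeats a few components and includes two moves with no component connected.
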(event EventBeginPlay
  (Utilities|FlowControl|Delay 5.0)
  (Class|BPIntPlatform|Camerashake(Message) (Game|GetPlayerCharacter 0))
  (Utilities|FlowControl|Delay 1.0)
  (Components|MoveComponentTo (Variables|Default|GetLandScape_Sphere_054) (Math|Vector|MakeVector 0.0 0.0 (Variables|Default|GetLocationZ)) "0, 0, 0" false false (Variables|Default|GetFalltime) false)
  (Utilities|FlowControl|Delay (Variables|Default|GetDelay_per_falling-object))
  (Components|MoveComponentTo (Variables|Default|GetLandScape_Sphere_003) (Math|Vector|MakeVector 0.0 0.0 (Variables|Default|GetLocationZ)) "0, 0, 0" false false (Variables|Default|GetFalltime) false)
  (Utilities|FlowControl|Delay (Variables|Default|GetDelay_per_falling-object))
  (Components|MoveComponentTo (Variables|Default|GetLandScape_Sphere_004) (Math|Vector|MakeVector 0.0 0.0 (Variables|Default|GetLocationZ)) "0, 0, 0" false false (Variables|Default|GetFalltime) false)
  (Utilities|FlowControl|Delay (Variables|Default|GetDelay_per_falling-object))
  (Components|MoveComponentTo (Variables|Default|GetLandScape_Sphere_034) (Math|Vector|MakeVector 0.0 0.0 (Variables|Default|GetLocationZ)) "0, 0, 0" false false (Variables|Default|GetFalltime) false)
  (Utilities|FlowControl|Delay (Variables|Default|GetDelay_per_falling-object))
  (Components|MoveComponentTo (Variables|Default|GetLandScape_Sphere_002) (Math|Vector|MakeVector 0.0 0.0 (Variables|Default|GetLocationZ)) "0, 0, 0" false false (Variables|Default|GetFalltime) false)
  (Utilities|FlowControl|Delay 15.0)
  (Class|BPIntPlatform|Camerashake(Message) (Game|GetPlayerCharacter 0))
  (Utilities|FlowControl|Delay 1.0)
  (Utilities|FlowControl|Delay (Variables|Default|GetDelay_per_falling-object))
  (Components|MoveComponentTo (Variables|Default|GetLandScape_Sphere_001) (Math|Vector|MakeVector 0.0 0.0 (Variables|Default|GetLocationZ)) "0, 0, 0" false false (Variables|Default|GetFalltime) false)
  (Utilities|FlowControl|Delay (Variables|Default|GetDelay_per_falling-object))
  (Components|MoveComponentTo (Variables|Default|GetLandScape_Sphere_051) (Math|Vector|MakeVector 0.0 0.0 (Variables|Default|GetLocationZ)) "0, 0, 0" false false (Variables|Default|GetFalltime) false)
  (Utilities|FlowControl|Delay (Variables|Default|GetDelay_per_falling-object))
  (Components|MoveComponentTo (Variables|Default|GetLandScape_Sphere_048) (Math|Vector|MakeVector 0.0 0.0 (Variables|Default|GetLocationZ)) "0, 0, 0" false false (Variables|Default|GetFalltime) false)
  (Utilities|FlowControl|Delay (Variables|Default|GetDelay_per_falling-object))
  (Components|MoveComponentTo (Variables|Default|GetLandScape_Sphere_045) (Math|Vector|MakeVector 0.0 0.0 (Variables|Default|GetLocationZ)) "0, 0, 0" false false (Variables|Default|GetFalltime) false)
  (Utilities|FlowControl|Delay (Variables|Default|GetDelay_per_falling-object))
  (Components|MoveComponentTo (Variables|Default|GetLandScape_Sphere_040) (Math|Vector|MakeVector 0.0 0.0 (Variables|Default|GetLocationZ)) "0, 0, 0" false false (Variables|Default|GetFalltime) false)
  (Utilities|FlowControl|Delay 15.0)
  (Utilities|FlowControl|Delay (Variables|Default|GetDelay_per_falling-object))
  (Components|MoveComponentTo (Variables|Default|GetLandScape_Sphere_028) (Math|Vector|MakeVector 0.0 0.0 (Variables|Default|GetLocationZ)) "0, 0, 0" false false (Variables|Default|GetFalltime) false)
  (Utilities|FlowControl|Delay (Variables|Default|GetDelay_per_falling-object))
  (Components|MoveComponentTo (Variables|Default|GetLandScape_Sphere_044) (Math|Vector|MakeVector 0.0 0.0 (Variables|Default|GetLocationZ)) "0, 0, 0" false false (Variables|Default|GetFalltime) false)
  (Utilities|FlowControl|Delay (Variables|Default|GetDelay_per_falling-object))
  (Components|MoveComponentTo (Variables|Default|GetLandScape_Sphere_009) (Math|Vector|MakeVector 0.0 0.0 (Variables|Default|GetLocationZ)) "0, 0, 0" false false (Variables|Default|GetFalltime) false)
  (Utilities|FlowControl|Delay (Variables|Default|GetDelay_per_falling-object))
  (Components|MoveComponentTo (Variables|Default|GetLandScape_Sphere_041) (Math|Vector|MakeVector 0.0 0.0 (Variables|Default|GetLocationZ)) "0, 0, 0" false false (Variables|Default|GetFalltime) false)
  (Utilities|FlowControl|Delay (Variables|Default|GetDelay_per_falling-object))
  (Components|MoveComponentTo (Variables|Default|GetLandScape_Sphere_028) (Math|Vector|MakeVector 0.0 0.0 (Variables|Default|GetLocationZ)) "0, 0, 0" false false (Variables|Default|GetFalltime) false)
  (Utilities|FlowControl|Delay (Variables|Default|GetDelay_per_falling-object))
  (Components|MoveComponentTo (Variables|Default|GetLandScape_Sphere_037) (Math|Vector|MakeVector 0.0 0.0 (Variables|Default|GetLocationZ)) "0, 0, 0" false false (Variables|Default|GetFalltime) false)
  (Utilities|FlowControl|Delay (Variables|Default|GetDelay_per_falling-object))
  (Components|MoveComponentTo (Variables|Default|GetLandScape_Sphere_039) (Math|Vector|MakeVector 0.0 0.0 (Variables|Default|GetLocationZ)) "0, 0, 0" false false (Variables|Default|GetFalltime) false)
  (Utilities|FlowControl|Delay (Variables|Default|GetDelay_per_falling-object))
  (Components|MoveComponentTo (Variables|Default|GetLandScape_Sphere_035) (Math|Vector|MakeVector 0.0 0.0 (Variables|Default|GetLocationZ)) "0, 0, 0" false false (Variables|Default|GetFalltime) false)
  (Utilities|FlowControl|Delay (Variables|Default|GetDelay_per_falling-object))
  (Components|MoveComponentTo (Variables|Default|GetLandScape_Sphere_009) (Math|Vector|MakeVector 0.0 0.0 (Variables|Default|GetLocationZ)) "0, 0, 0" false false (Variables|Default|GetFalltime) false)
  (Utilities|FlowControl|Delay (Variables|Default|GetDelay_per_falling-object))
  (Components|MoveComponentTo (Variables|Default|GetLandScape_Sphere_058) (Math|Vector|MakeVector 0.0 0.0 (Variables|Default|GetLocationZ)) "0, 0, 0" false false (Variables|Default|GetFalltime) false)
  (Utilities|FlowControl|Delay (Variables|Default|GetDelay_per_falling-object))
  (Components|MoveComponentTo (Variables|Default|GetLandScape_Sphere_031) (Math|Vector|MakeVector 0.0 0.0 (Variables|Default|GetLocationZ)) "0, 0, 0" false false (Variables|Default|GetFalltime) false)
  (Utilities|FlowControl|Delay (Variables|Default|GetDelay_per_falling-object))
  (Components|MoveComponentTo (Variables|Default|GetLandScape_Sphere_031) (Math|Vector|MakeVector 0.0 0.0 (Variables|Default|GetLocationZ)) "0, 0, 0" false false (Variables|Default|GetFalltime) false)
  (Utilities|FlowControl|Delay (Variables|Default|GetDelay_per_falling-object))
  (Components|MoveComponentTo (Variables|Default|GetLandScape_Sphere_042) (Math|Vector|MakeVector 0.0 0.0 (Variables|Default|GetLocationZ)) "0, 0, 0" false false (Variables|Default|GetFalltime) false)
  (Utilities|FlowControl|Delay (Variables|Default|GetDelay_per_falling-object))
  (Components|MoveComponentTo (Variables|Default|GetLandScape_Sphere_043) (Math|Vector|MakeVector 0.0 0.0 (Variables|Default|GetLocationZ)) "0, 0, 0" false false (Variables|Default|GetFalltime) false)
  (Utilities|FlowControl|Delay (Variables|Default|GetDelay_per_falling-object))
  (Components|MoveComponentTo (Variables|Default|GetLandScape_Sphere_060) (Math|Vector|MakeVector 0.0 0.0 (Variables|Default|GetLocationZ)) "0, 0, 0" false false (Variables|Default|GetFalltime) false)
  (Utilities|FlowControl|Delay (Variables|Default|GetDelay_per_falling-object))
  (Components|MoveComponentTo (Variables|Default|GetLandScape_Sphere_010) (Math|Vector|MakeVector 0.0 0.0 (Variables|Default|GetLocationZ)) "0, 0, 0" false false (Variables|Default|GetFalltime) false)
  (Utilities|FlowControl|Delay (Variables|Default|GetDelay_per_falling-object))
  (Components|MoveComponentTo (Variables|Default|GetLandScape_Sphere_061) (Math|Vector|MakeVector 0.0 0.0 (Variables|Default|GetLocationZ)) "0, 0, 0" false false (Variables|Default|GetFalltime) false)
  (Utilities|FlowControl|Delay (Variables|Default|GetDelay_per_falling-object))
  (Components|MoveComponentTo (Variables|Default|GetLandScape_Sphere_064) (Math|Vector|MakeVector 0.0 0.0 (Variables|Default|GetLocationZ)) "0, 0, 0" false false (Variables|Default|GetFalltime) false)
  (Utilities|FlowControl|Delay (Variables|Default|GetDelay_per_falling-object))
  (Components|MoveComponentTo (Variables|Default|GetLandScape_Sphere_011) (Math|Vector|MakeVector 0.0 0.0 (Variables|Default|GetLocationZ)) "0, 0, 0" false false (Variables|Default|GetFalltime) false)
  (Utilities|FlowControl|Delay (Variables|Default|GetDelay_per_falling-object))
  (Components|MoveComponentTo (Variables|Default|GetLandScape_Sphere_062) (Math|Vector|MakeVector 0.0 0.0 (Variables|Default|GetLocationZ)) "0, 0, 0" false false (Variables|Default|GetFalltime) false)
  (Utilities|FlowControl|Delay (Variables|Default|GetDelay_per_falling-object))
  (Components|MoveComponentTo (Variables|Default|GetLandScape_Sphere_063) (Math|Vector|MakeVector 0.0 0.0 (Variables|Default|GetLocationZ)) "0, 0, 0" false false (Variables|Default|GetFalltime) false)
  (Utilities|FlowControl|Delay (Variables|Default|GetDelay_per_falling-object))
  (Components|MoveComponentTo (Variables|Default|GetLandScape_Sphere_018) (Math|Vector|MakeVector 0.0 0.0 (Variables|Default|GetLocationZ)) "0, 0, 0" false false (Variables|Default|GetFalltime) false)
  (Utilities|FlowControl|Delay (Variables|Default|GetDelay_per_falling-object))
  (Components|MoveComponentTo (Variables|Default|GetLandScape_Sphere_036) (Math|Vector|MakeVector 0.0 0.0 (Variables|Default|GetLocationZ)) "0, 0, 0" false false (Variables|Default|GetFalltime) false)
  (Utilities|FlowControl|Delay (Variables|Default|GetDelay_per_falling-object))
  (Components|MoveComponentTo (Variables|Default|GetLandScape_Sphere_022) (Math|Vector|MakeVector 0.0 0.0 (Variables|Default|GetLocationZ)) "0, 0, 0" false false (Variables|Default|GetFalltime) false)
  (Utilities|FlowControl|Delay (Variables|Default|GetDelay_per_falling-object))
  (Components|MoveComponentTo (Variables|Default|GetLandScape_Sphere_038) (Math|Vector|MakeVector 0.0 0.0 (Variables|Default|GetLocationZ)) "0, 0, 0" false false (Variables|Default|GetFalltime) false)
  (Utilities|FlowControl|Delay (Variables|Default|GetDelay_per_falling-object))
  (Components|MoveComponentTo (Variables|Default|GetLandScape_Sphere_008) (Math|Vector|MakeVector 0.0 0.0 (Variables|Default|GetLocationZ)) "0, 0, 0" false false (Variables|Default|GetFalltime) false)
  (Utilities|FlowControl|Delay (Variables|Default|GetDelay_per_falling-object))
  (Components|MoveComponentTo (Variables|Default|GetLandScape_Sphere_046) (Math|Vector|MakeVector 0.0 0.0 (Variables|Default|GetLocationZ)) "0, 0, 0" false false (Variables|Default|GetFalltime) false)
  (Utilities|FlowControl|Delay (Variables|Default|GetDelay_per_falling-object))
  (Components|MoveComponentTo (Variables|Default|GetLandScape_Sphere_047) (Math|Vector|MakeVector 0.0 0.0 (Variables|Default|GetLocationZ)) "0, 0, 0" false false (Variables|Default|GetFalltime) false)
  (Utilities|FlowControl|Delay (Variables|Default|GetDelay_per_falling-object))
  (Components|MoveComponentTo (Variables|Default|GetLandScape_Sphere_025) (Math|Vector|MakeVector 0.0 0.0 (Variables|Default|GetLocationZ)) "0, 0, 0" false false (Variables|Default|GetFalltime) false)
  (Utilities|FlowControl|Delay (Variables|Default|GetDelay_per_falling-object))
  (Components|MoveComponentTo (Variables|Default|GetLandScape_Sphere_007) (Math|Vector|MakeVector 0.0 0.0 (Variables|Default|GetLocationZ)) "0, 0, 0" false false (Variables|Default|GetFalltime) false)
  (Utilities|FlowControl|Delay (Variables|Default|GetDelay_per_falling-object))
  (Components|MoveComponentTo (Variables|Default|GetLandScape_Sphere_033) (Math|Vector|MakeVector 0.0 0.0 (Variables|Default|GetLocationZ)) "0, 0, 0" false false (Variables|Default|GetFalltime) false)
  (Utilities|FlowControl|Delay (Variables|Default|GetDelay_per_falling-object))
  (Components|MoveComponentTo (Variables|Default|GetLandScape_Sphere_059) (Math|Vector|MakeVector 0.0 0.0 (Variables|Default|GetLocationZ)) "0, 0, 0" false false (Variables|Default|GetFalltime) false)
  (Utilities|FlowControl|Delay (Variables|Default|GetDelay_per_falling-object))
  (Components|MoveComponentTo (Variables|Default|GetLandScape_Sphere_057) (Math|Vector|MakeVector 0.0 0.0 (Variables|Default|GetLocationZ)) "0, 0, 0" false false (Variables|Default|GetFalltime) false)
  (Utilities|FlowControl|Delay (Variables|Default|GetDelay_per_falling-object))
  (Components|MoveComponentTo (Variables|Default|GetLandScape_Sphere_053) (Math|Vector|MakeVector 0.0 0.0 (Variables|Default|GetLocationZ)) "0, 0, 0" false false (Variables|Default|GetFalltime) false)
  (Utilities|FlowControl|Delay (Variables|Default|GetDelay_per_falling-object))
  (Components|MoveComponentTo (Variables|Default|GetLandScape_Sphere_050) (Math|Vector|MakeVector 0.0 0.0 (Variables|Default|GetLocationZ)) "0, 0, 0" false false (Variables|Default|GetFalltime) false)
  (Utilities|FlowControl|Delay (Variables|Default|GetDelay_per_falling-object))
  (Components|MoveComponentTo (Variables|Default|GetLandScape_Sphere_006) (Math|Vector|MakeVector 0.0 0.0 (Variables|Default|GetLocationZ)) "0, 0, 0" false false (Variables|Default|GetFalltime) false)
  (Utilities|FlowControl|Delay (Variables|Default|GetDelay_per_falling-object))
  (Components|MoveComponentTo (Variables|Default|GetLandScape_Sphere_021) (Math|Vector|MakeVector 0.0 0.0 (Variables|Default|GetLocationZ)) "0, 0, 0" false false (Variables|Default|GetFalltime) false)
  (Utilities|FlowControl|Delay (Variables|Default|GetDelay_per_falling-object))
  (Components|MoveComponentTo (Variables|Default|GetLandScape_Sphere_024) (Math|Vector|MakeVector 0.0 0.0 (Variables|Default|GetLocationZ)) "0, 0, 0" false false (Variables|Default|GetFalltime) false)
  (Utilities|FlowControl|Delay (Variables|Default|GetDelay_per_falling-object))
  (Components|MoveComponentTo (Variables|Default|GetLandScape_Sphere_027) (Math|Vector|MakeVector 0.0 0.0 (Variables|Default|GetLocationZ)) "0, 0, 0" false false (Variables|Default|GetFalltime) false)
  (Utilities|FlowControl|Delay (Variables|Default|GetDelay_per_falling-object))
  (Components|MoveComponentTo (Variables|Default|GetLandScape_Sphere_030) (Math|Vector|MakeVector 0.0 0.0 (Variables|Default|GetLocationZ)) "0, 0, 0" false false (Variables|Default|GetFalltime) false)
  (Utilities|FlowControl|Delay (Variables|Default|GetDelay_per_falling-object))
  (Components|MoveComponentTo (Variables|Default|GetLandScape_Sphere_005) (Math|Vector|MakeVector 0.0 0.0 (Variables|Default|GetLocationZ)) "0, 0, 0" false false (Variables|Default|GetFalltime) false)
  (Utilities|FlowControl|Delay (Variables|Default|GetDelay_per_falling-object))
  (Components|MoveComponentTo 0 (Math|Vector|MakeVector 0.0 0.0 (Variables|Default|GetLocationZ)) "0, 0, 0" false false (Variables|Default|GetFalltime) false)
  (Utilities|FlowControl|Delay (Variables|Default|GetDelay_per_falling-object))
  (Components|MoveComponentTo 0 (Math|Vector|MakeVector 0.0 0.0 (Variables|Default|GetLocationZ)) "0, 0, 0" false false (Variables|Default|GetFalltime) false)
  (Utilities|FlowControl|Delay (Variables|Default|GetDelay_per_falling-object))
  (Components|MoveComponentTo (Variables|Default|GetLandScape_Sphere_019) (Math|Vector|MakeVector 0.0 0.0 (Variables|Default|GetLocationZ)) "0, 0, 0" false false (Variables|Default|GetFalltime) false)
  (Utilities|FlowControl|Delay (Variables|Default|GetDelay_per_falling-object))
  (Components|MoveComponentTo (Variables|Default|GetLandScape_Sphere_032) (Math|Vector|MakeVector 0.0 0.0 (Variables|Default|GetLocationZ)) "0, 0, 0" false false (Variables|Default|GetFalltime) false))

(fn ConstructionScript)