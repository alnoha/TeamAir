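; Main game mode for a local multiplayer last-player-standing match.
; BeginPlay replaces existing characters with possessed, color-coded ones, creates local players, sets a shared gameplay camera and disables input.
; StartMatch shows a countdown widget that re-enables input when finished.
; PlayerDied trims the remaining list; at one or fewer, GameEnded fires once with slow motion, fanfare, win screen and a camera blend to the winner.
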(event Custom|GameEnded
  (bind _returnvalue (Game|GetPlayerController 0))
  (Utilities|FlowControl|DoOnce false
    (:Completed
      (bind _returnvalue_2 (UserInterface|CreateWidget "/Game/Core/UI/UI_WinScreen.UI_WinScreen_C" 0 (Class|GameplayStatics|GetPlayerControllerID (.AsPC (Utilities|Casting|CastToPC (Pawn|GetController (Utilities|Array|Get(acopy) (Variables|Default|GetPlayersRemaining))))))))
      (UserInterface|Viewport|AddtoViewport _returnvalue_2 0)
      (Utilities|FlowControl|Sequence
        (:then_0
          (Audio|PlaySound2D "/Game/Audio/Interface/Winn.Winn" 1.0 1.0 0.0 0 0)
          (Utilities|Time|SetGlobalTimeDilation 0.1)
          (Audio|PlaySound2D "/Game/Audio/Music/Fanfares_Win_02.Fanfares_Win_02" 1.0 1.0 0.0 0 0))
        (:then_1
          (Input|SetInputModeUIOnly _returnvalue _returnvalue_2 "DoNotLock")
          (Variables|/Script/Engine.PlayerController|SetbShowMouseCursor _returnvalue true))
        (:then_2
          (Game|Player|SetViewTargetwithBlend (Game|GetPlayerController 0) (Utilities|Array|Get(acopy) (Variables|Default|GetPlayersRemaining)) 0.1 "VTBlend_EaseInOut" 2.0 true))))))

(event Custom|Start%20Match
  ;[1 1 1] Match Start
  (bind _returnvalue (UserInterface|CreateWidget "/Game/UI/UI_MatchCountdown.UI_MatchCountdown_C"))
  (UserInterface|Viewport|AddtoViewport _returnvalue 0)
  (EventDispatchers|BindEventtoCountdownFinished _returnvalue (delegate Custom|Match%20Begin)))

(event Custom|Match%20Begin
  ;[1 1 1] Match Start
  (CallFunction|ToggleInput true))

(event EventBeginPlay
  (Utilities|FlowControl|Sequence
    (:then_0
      ;[1 1 1] Destroy preexisting characters (dirty fix)
      (bind _outactors (Actor|GetAllActorsOfClass "/Game/Core/PlayerChar.PlayerChar_C"))
      (for _array_element _outactors
        (Actor|DestroyActor _array_element)))
    (:then_1
      (bind _outactors_2 (Actor|GetAllActorsOfClass "/Game/Core/PC.PC_C"))
      (for (_array_element_2 _array_index) _outactors_2
        (if (< _array_index (Variables|/Game/Core/GI.GI_C|GetNumPlayers (.AsGI (Utilities|Casting|CastToGI (Game|GetGameInstance)))))
          (bind _returnvalue (Game|SpawnActorfromClass "/Game/Core/PlayerChar.PlayerChar_C" (Math|Transform|MakeTransform "0, 0,10000.000000" "0, 0, 0" "1,1,1") "AlwaysSpawn" 0 0))
          (Pawn|Possess _array_element_2 _returnvalue)
          (Variables|/Game/Core/PC.PC_C|SetPlayer%20Index _array_element_2 _array_index)
          (Utilities|Array|AddUnique (Variables|Default|GetPlayers) _array_element_2)
          (bind _asplayer_char (Utilities|Casting|CastToPlayerChar (Pawn|GetControlledPawn _array_element_2)))
          (Utilities|Array|AddUnique (Variables|Default|GetPlayersRemaining) _asplayer_char)
          (Default|SetColor _asplayer_char _array_index))))
    (:then_2
      ;[1 1 1] Add Players
      (for _index (range 0 (- (Variables|/Game/Core/GI.GI_C|GetNumPlayers (.AsGI (Utilities|Casting|CastToGI (Game|GetGameInstance)))) 1))
        (bind _returnvalue_2 (Class|GameplayStatics|CreatePlayer -1))
        (Utilities|Casting|CastToPC _returnvalue_2)))
    (:then_3
      ;[1 1 1] Go To Gameplay Camera
      (bind _outactors_3 (Actor|GetAllActorsOfClass "/Game/Camera/GameplayCamera.GameplayCamera_C"))
      (Game|Player|SetViewTargetwithBlend (Game|GetPlayerController 0) (Utilities|Array|Get(acopy) _outactors_3) 0.0 "VTBlend_Linear" 0.0 false))
    (:then_4
      (bind _outactors_4 (Actor|GetAllActorsOfClass "/Game/Core/PlayerChar.PlayerChar_C"))
      (for _array_element_3 _outactors_4
        (if (not (Class|Pawn|IsControlled _array_element_3))
          (Actor|DestroyActor _array_element_3))))
    (:then_5
      ;[1 1 1] Start MAtch
      (Variables|Default|SetMatchStarted true))
    (:then_6
      ;[1 1 1] Disable Input on start
      (CallFunction|ToggleInput false))))

(event EventPlayerDied
  (params (PlayerCharacter :type Player%20Char%20Object%20Reference))
  (bind _playersremaining (Variables|Default|GetPlayersRemaining))
  (if (Variables|Default|GetMatchStarted)
    (Utilities|Array|RemoveItem _playersremaining PlayerCharacter)
    (Math|Integer|CompareInt (Utilities|Array|Length _playersremaining) 1
      (:>
        ;[1 1 1] Go To Gameplay Camera
        (bind _outactors (Actor|GetAllActorsOfClass "/Game/Camera/GameplayCamera.GameplayCamera_C"))
        (Game|Player|SetViewTargetwithBlend (Game|GetPlayerController 0) (Utilities|Array|Get(acopy) _outactors) 0.0 "VTBlend_Linear" 0.0 false))
      (:==
        (CallFunction|GameEnded :!label _label))
      (:<
        (goto _label)))))

(fn ConstructionScript)

(fn ToggleInput
  (params (Enabled :type Boolean))
  (bind _outactors (Actor|GetAllActorsOfClass "/Script/Engine.PlayerController"))
  (for _array_element _outactors
    (if Enabled
      (Input|EnableInput _array_element _array_element)
      (else
        (Input|DisableInput _array_element _array_element)))))