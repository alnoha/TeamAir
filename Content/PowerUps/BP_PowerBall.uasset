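; BP_PowerBall is a power-up pickup ball that spins in place and reacts when the player touches it.
; A Spin timeline started on BeginPlay adds a fixed yaw step to the sphere on each update, so its speed depends on frame rate.
; Overlapping the sphere collider with a PlayerChar stores it as AffectedCharacter and calls PickUp, which is empty here.
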(event OnComponentBeginOverlap(SphereCollider)
  (params (OverlappedComponent :type Primitive%20Component%20Object%20Reference) (OtherActor :type Actor%20Object%20Reference) (OtherComp :type Primitive%20Component%20Object%20Reference) (OtherBodyIndex :type Integer) (bFromSweep :type Boolean) (SweepResult :type Hit%20Result%20Structure%20%28by%20ref%29))
  (if (== (Utilities|GetClass OtherActor) "/Game/Core/PlayerChar.PlayerChar_C")
    (bind _asplayer_char (Utilities|Casting|CastToPlayerChar OtherActor))
    (Variables|Default|SetAffected%20character _asplayer_char)
    (CallFunction|PickUp)))

(event Custom|PickUp)

(event EventBeginPlay
  (bind _sphere (Variables|Default|GetSphere))
  (Timeline|Spin PlayFromStart
    (:Update
      (Transformation|SetWorldRotation _sphere (Math|Rotator|MakeRotator 0.0 0.0 (+ (.yaw (Transformation|GetWorldRotation _sphere)) 1.0)) false false))))

(fn ConstructionScript)