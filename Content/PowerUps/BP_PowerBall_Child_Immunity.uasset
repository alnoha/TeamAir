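; Immunity power-up ball, a power-ball child that makes the character picking it up temporarily immune to damage.
; After the parent pickup logic, it blocks damage, activates immunity particles and tints the character's power-up light orange-red with a wider radius.
; An event track on the Immunity timeline reverts these effects, while a second timeline ends a global slow-motion effect.
; The ball hides, disables collision and destroys itself after a short delay.
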(event EventPickUp
  (bind _affected_character (Variables|Default|GetAffected%20character))
  (bind _poweruplight (Variables|/Game/Core/PlayerChar.PlayerChar_C|GetPowerUpLight _affected_character))
  (bind _particleimmunity (Variables|/Game/Core/PlayerChar.PlayerChar_C|GetParticleImmunity _affected_character))
  (|CallParentFunction)
  (Utilities|FlowControl|Sequence
    (:then_0
      (Components|Activation|Activate _particleimmunity false)
      (Default|PreventDamage _affected_character)
      (Rendering|Components|Light|SetLightColor _poweruplight "(R=1.000000,G=0.069188,B=0.000000,A=1.000000)" true)
      (Rendering|Lighting|SetAttenuationRadius _poweruplight 1.5e+02)
      (Timeline|Immunity PlayFromStart
        (:ImmunityTimer
          (Default|AllowDamage _affected_character)
          (Rendering|Components|Light|SetLightColor _poweruplight "(R=1.000000,G=1.000000,B=1.000000,A=1.000000)" true)
          (Rendering|Lighting|SetAttenuationRadius _poweruplight 1.2e+02)
          (Components|Activation|Deactivate _particleimmunity))))
    (:then_1
      (Utilities|Time|SetGlobalTimeDilation 0.6)
      (Timeline|DilationTimeline PlayFromStart
        (:Duration
          (Utilities|Time|SetGlobalTimeDilation 1.0))))
    (:then_2
      (Rendering|SetVisibility (Variables|Default|GetDefaultSceneRoot) false true)
      (Collision|SetCollisionEnabled (Variables|Default|GetSphereCollider) "NoCollision")
      (Utilities|FlowControl|Delay 3.0)
      (Actor|DestroyActor))))

(fn ConstructionScript
  (|CallParentFunction))