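; Quick variant of the PowerBall power-up, granting a temporary speed boost to the character that picks it up.
; On PickUp it runs the parent logic, raises the affected character's max walk speed and slows global time.
; Two timelines act as timers through event tracks: one sets walk speed back to a fixed value, the other restores normal time dilation and destroys the ball.
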(event EventBeginPlay)

(event Collision|EventActorBeginOverlap
  (params (OtherActor :type Actor%20Object%20Reference))
  (|CallParentFunction OtherActor) ; This node is disabled and will not be called.\nDrag off pins to build functionality.
)

(event EventTick
  (params (DeltaSeconds :type Float%20%28single-precision%29)))

(event EventPickUp
  (bind _affected_character (Variables|Default|GetAffected%20character))
  (|CallParentFunction)
  (Utilities|FlowControl|Sequence
    (:then_0
      (Development|PrintString "Speed Up!" true true "(R=0.000000,G=0.660000,B=1.000000,A=1.000000)" 5.0)
      (Variables|/Script/Engine.CharacterMovementComponent|SetMaxWalkSpeed (Variables|/Script/Engine.Character|GetCharacterMovement _affected_character) 1e+03)
      (Timeline|IncreaseSpeed PlayFromStart
        (:3%20seconds
          (Variables|/Script/Engine.CharacterMovementComponent|SetMaxWalkSpeed (Variables|/Script/Engine.Character|GetCharacterMovement _affected_character) 6e+02))))
    (:then_1
      (Utilities|Time|SetGlobalTimeDilation 0.6)
      (Timeline|Timeline_0 PlayFromStart
        (:Duration
          (Utilities|Time|SetGlobalTimeDilation 1.0)
          (Actor|DestroyActor))))))

(fn ConstructionScript
  (|CallParentFunction))