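; BP_PowerBall_Child_ShieldCharge is a power-up pickup that grants the affected character one extra Block, apparently a shield charge.
; After the parent pickup logic, it briefly activates the character's heal particles and tints and widens their power-up light.
; It also slows global time until a timeline event restores normal speed.
; The ball hides and disables collision immediately, delaying destruction so the timed effects can run.
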(event EventPickUp
  (bind _affected_character (Variables|Default|GetAffected%20character))
  (bind _poweruplight (Variables|/Game/Core/PlayerChar.PlayerChar_C|GetPowerUpLight _affected_character))
  (bind _particleheal (Variables|/Game/Core/PlayerChar.PlayerChar_C|GetParticleHeal _affected_character))
  (|CallParentFunction)
  (Utilities|FlowControl|Sequence
    (:then_0
      (Components|Activation|Activate _particleheal false)
      (Variables|/Game/Core/PlayerChar.PlayerChar_C|SetBlocks _affected_character (+ (Variables|/Game/Core/PlayerChar.PlayerChar_C|GetBlocks _affected_character) 1))
      (Rendering|Components|Light|SetLightColor _poweruplight "(R=1.000000,G=0.616479,B=0.000000,A=1.000000)" true)
      (Rendering|Lighting|SetAttenuationRadius _poweruplight 1.5e+02)
      (Utilities|FlowControl|Delay 1.0)
      (Rendering|Components|Light|SetLightColor _poweruplight "(R=1.000000,G=1.000000,B=1.000000,A=1.000000)" true)
      (Rendering|Lighting|SetAttenuationRadius _poweruplight 1.2e+02)
      (Components|Activation|Deactivate _particleheal))
    (:then_1
      (Utilities|Time|SetGlobalTimeDilation 0.6)
      (Timeline|Timeline_0 PlayFromStart
        (:Duration
          (Utilities|Time|SetGlobalTimeDilation 1.0))))
    (:then_2
      (Rendering|SetVisibility (Variables|Default|GetDefaultSceneRoot) false true)
      (Collision|SetCollisionEnabled (Variables|Default|GetSphereCollider) "NoCollision")
      (Utilities|FlowControl|Delay 3.0)
      (Actor|DestroyActor))))

(fn ConstructionScript
  (|CallParentFunction))