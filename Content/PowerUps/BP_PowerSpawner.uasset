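; Power-up spawner that, after a delay at BeginPlay, periodically spawns actors at its own height using the level's PlatformBlocks.
; The TL_Spawner timeline event picks a random block and, if it has not fallen, runs one of five random spawn branches, then restarts the timeline.
; Four branches re-roll blocks separately for X and Y, so spawns can miss the checked block; the fifth sets only Z.
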(event EventBeginPlay
  (bind _returnvalue (Transformation|GetActorLocation))
  (bind _returnvalue_2 (Transformation|GetActorScale3D))
  (Utilities|FlowControl|Delay 1e+01)
  (Timeline|TL_Spawner PlayFromStart
    (:SpawnFirst
      (bind _outactors (Actor|GetAllActorsOfClass "/Game/LevelBP/NewPlatform/Hexagon/PlatformBlock.PlatformBlock_C"))
      (Variables|Default|SetBlockRef (Utilities|Array|Get(acopy) _outactors (Math|Random|RandomInteger (Utilities|Array|LastIndex _outactors))))
      (Utilities|IsValid (Variables|Default|GetBlockRef)
        (:Is%20Valid
          (if (not (Variables|/Game/LevelBP/NewPlatform/Hexagon/PlatformBlock.PlatformBlock_C|GethasFallen (Variables|Default|GetBlockRef)))
            (switch int (Math|Random|RandomIntegerinRange 0 4)
              (:0
                (Game|SpawnActorfromClass "/Game/PowerUps/BP_PowerBall_Child_Immunity.BP_PowerBall_Child_Immunity_C" (Math|Transform|MakeTransform (Math|Vector|MakeVector (.x (Transformation|GetActorLocation (Utilities|Array|Get(acopy) _outactors (Math|Random|RandomInteger (Utilities|Array|LastIndex _outactors))))) (.y (Transformation|GetActorLocation (Utilities|Array|Get(acopy) _outactors (Math|Random|RandomInteger (Utilities|Array|LastIndex _outactors))))) (.z _returnvalue)) "0, 0, 0" _returnvalue_2) "Undefined" 0 0)
                (Timeline|TL_Spawner PlayFromStart))
              (:1
                (Game|SpawnActorfromClass "/Game/PowerUps/BP_PowerBall_Child_Quick.BP_PowerBall_Child_Quick_C" (Math|Transform|MakeTransform (Math|Vector|MakeVector (.x (Transformation|GetActorLocation (Utilities|Array|Get(acopy) _outactors (Math|Random|RandomInteger (Utilities|Array|LastIndex _outactors))))) (.y (Transformation|GetActorLocation (Utilities|Array|Get(acopy) _outactors (Math|Random|RandomInteger (Utilities|Array|LastIndex _outactors))))) (.z _returnvalue)) "0, 0, 0" _returnvalue_2) "Undefined" 0 0)
                (Timeline|TL_Spawner PlayFromStart))
              (:2
                (Game|SpawnActorfromClass "/Game/PowerUps/BP_PowerBall_Child_Health.BP_PowerBall_Child_Health_C" (Math|Transform|MakeTransform (Math|Vector|MakeVector (.x (Transformation|GetActorLocation (Utilities|Array|Get(acopy) _outactors (Math|Random|RandomInteger (Utilities|Array|LastIndex _outactors))))) (.y (Transformation|GetActorLocation (Utilities|Array|Get(acopy) _outactors (Math|Random|RandomInteger (Utilities|Array|LastIndex _outactors))))) (.z _returnvalue)) "0, 0, 0" _returnvalue_2) "Undefined" 0 0)
                (Timeline|TL_Spawner PlayFromStart))
              (:3
                (Game|SpawnActorfromClass "/Game/PowerUps/BP_PowerBall_Child_Dash.BP_PowerBall_Child_Dash_C" (Math|Transform|MakeTransform (Math|Vector|MakeVector (.x (Transformation|GetActorLocation (Utilities|Array|Get(acopy) _outactors (Math|Random|RandomInteger (Utilities|Array|LastIndex _outactors))))) (.y (Transformation|GetActorLocation (Utilities|Array|Get(acopy) _outactors (Math|Random|RandomInteger (Utilities|Array|LastIndex _outactors))))) (.z _returnvalue)) "0, 0, 0" _returnvalue_2) "Undefined" 0 0)
                (Timeline|TL_Spawner PlayFromStart))
              (:4
                (Game|SpawnActorfromClass "/Game/PowerUps/BP_PowerBall_Child_ShieldCharge.BP_PowerBall_Child_ShieldCharge_C" (Math|Transform|MakeTransform (Math|Vector|MakeVector 0.0 0.0 (.z _returnvalue)) "0, 0, 0" _returnvalue_2) "Undefined" 0 0)
                (Timeline|TL_Spawner PlayFromStart)))))))))

(fn ConstructionScript)